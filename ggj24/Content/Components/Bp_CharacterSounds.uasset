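; Character component that plays one-shot sound effects for attack, tackle start, jump, land and hurt events.
; On BeginPlay it adds an audio component to its owner if it has no valid one.
; Each event passes a random entry from its sound array to PlayOneShot, which swaps the sound on that single shared audio component and plays it.
; Tackle end and idle start events are empty stubs.
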(event `self.ReceiveBeginPlay`
  (`self.SetupAudio`))

(event `EventAttack`
  (`self.PlayOneShot` (`KismetArrayLibrary.Array_Random` (`self.AttackSound`))))

(event `EventTackleStart`
  (`self.PlayOneShot` (`KismetArrayLibrary.Array_Random` (`self.TackleSound`))))

(event `EventTackleEnd`)

(event `EventJump`
  (`self.PlayOneShot` (`KismetArrayLibrary.Array_Random` (`self.JumpSound`))))

(event `EventLand`
  (`self.PlayOneShot` (`KismetArrayLibrary.Array_Random` (`self.LandSound`))))

(event `EventHurt`
  (`self.PlayOneShot` (`KismetArrayLibrary.Array_Random` (`self.HurtSound`))))

(event `EventIdleStart`)

(fn `PlayOneShot`
  (params (Sound :type "SoundWave Object Reference"))
  (bind _audiocomponent (`self.AudioComponent`))
  (`AudioComponent.SetSound` _audiocomponent Sound)
  (`AudioComponent.Play` _audiocomponent 0.0))

(fn `SetupAudio`
  ;[1 1 1] CheckIfComponent exists
  (if (not (`KismetSystemLibrary.IsValid` (`self.AudioComponent`)))
    ;[1 1 1] Create Component
    (bind _returnvalue (`|AddComponentByClass` :`self` (`self.GetOwner`) :`Class` "/Script/Engine.AudioComponent"))
    (set `self.AudioComponent` _returnvalue)))