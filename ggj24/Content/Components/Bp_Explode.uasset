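; Explosion component that applies knockback to characters and physics objects within a radius when its explode event fires.
; A sphere overlap gathers nearby actors; those with a CharacterMovementComponent get an impulse along their normalized position in Source's local space, scaled by strength and a player push multiplier.
; Other actors get a linear-falloff radial impulse on each primitive component, with a debug print.
; Separate dispatchers report character and object hits.
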(event `EventExplode`
  (bind _outactors (`KismetSystemLibrary.SphereOverlapActors` (`self.Sphere Pos`) (`self.Radius`) (`|MakeArray` "ObjectTypeQuery2" "ObjectTypeQuery4" "ObjectTypeQuery3" "ObjectTypeQuery5" "ObjectTypeQuery6" :!type "EObjectTypeQuery Enum")))
  (for _array_element _outactors
    (bind _returnvalue (`Actor.GetComponentByClass` _array_element "/Script/Engine.CharacterMovementComponent"))
    (if (`KismetSystemLibrary.IsValid` _returnvalue)
      (`CharacterMovementComponent.AddImpulse` _returnvalue (* (`KismetMathLibrary.Normal` (`KismetMathLibrary.InverseTransformLocation` (`Actor.GetTransform` (`self.Source`)) (`Actor.K2_GetActorLocation` _array_element))) (`self.Strength`) (`self.PlayerPushStrength`)) false)
      (`self.HandleCharacterExploded`)
      (else
        (for _array_element_2 (`Actor.K2_GetComponentsByClass` _array_element "/Script/Engine.PrimitiveComponent")
          (`PhysicsObjectBlueprintLibrary.ApplyRadialImpulse` _array_element_2 (`self.Sphere Pos`) (`self.Radius`) (`self.Strength`) "RIF_Linear")
          (`KismetSystemLibrary.PrintString` (`KismetStringLibrary.Concat_StrStr` "Exploded: " (`KismetStringLibrary.Conv_ObjectToString` _array_element_2)))
          (`self.HandleObjectExploded`))))))