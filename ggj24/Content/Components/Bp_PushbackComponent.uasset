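; Actor component that fires a radial pushback burst from an offset point on its owner.
; EventBurst sphere-overlaps nearby objects and impulses all their primitive components away from the point, adding the owner's velocity.
; The push direction is computed in each target's local space but applied as a world impulse.
; It also calls Bap on any Bp_BapTarget components, then fires HandleBurst.
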(event `EventBurst`
  (bind _returnvalue (`self.GetOwner`))
  (bind _returnvalue_2 (`KismetMathLibrary.TransformLocation` (`Actor.GetTransform` _returnvalue) (`self.TriggerSpherePoint`)))
  (bind _outactors (`KismetSystemLibrary.SphereOverlapActors` _returnvalue_2 (`self.Radius`) (`|MakeArray` "ObjectTypeQuery2" "ObjectTypeQuery4" "ObjectTypeQuery3" "ObjectTypeQuery5" "ObjectTypeQuery6" :!type "EObjectTypeQuery Enum") null (`|MakeArray` _returnvalue)))
  (`|ExecutionSequence`
    (:`then_0`
      (for _array_element _outactors
        (`|ExecutionSequence`
          (:`then_0`
            (for _array_element_2 (`Actor.K2_GetComponentsByClass` _array_element "/Script/Engine.PrimitiveComponent")
              (`PrimitiveComponent.AddImpulse` _array_element_2 (+ (* (`KismetMathLibrary.Normal` (`KismetMathLibrary.InverseTransformLocation` (`Actor.GetTransform` _array_element) _returnvalue_2)) (`self.BurstPower`) -1.0) (`Actor.GetVelocity` _returnvalue)) "None" false)))
          (:`then_1`
            (for _array_element_3 (`Actor.K2_GetComponentsByClass` _array_element "/Game/Components/Bp_BapTarget.Bp_BapTarget_C")
              (`/Game/Components/Bp_BapTarget.Bap` _array_element_3))))))
    (:`then_1`
      (`self.HandleBurst`))))