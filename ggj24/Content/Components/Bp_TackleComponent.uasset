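; Tackle component that attaches its owning actor to nearby actors through a physics constraint passed into its events.
; On tackle, it positions the constraint at a point relative to the owner, sphere-overlaps there, and constrains the owner's mesh to each hit actor's mesh in turn, reusing the single constraint.
; It then signals tackle start; release breaks the constraint and signals completion.
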(event `EventRelease`
  (params (Constraint :type "PhysicsConstraintComponent Object Reference"))
  (`PhysicsConstraintComponent.BreakConstraint` Constraint)
  (`self.HandleTackleComplete`))

(event `self.ReceiveTick`
  (params (DeltaSeconds :type "Float (single-precision)")))

(event `EventTackle`
  (params (Constraint :type "PhysicsConstraintComponent Object Reference"))
  (bind _returnvalue (`self.GetOwner`))
  (bind _returnvalue_2 (`Actor.GetTransform` _returnvalue))
  (bind _returnvalue_3 (`KismetMathLibrary.TransformLocation` _returnvalue_2 (`self.TriggerSpherePoint`)))
  (`PhysicsConstraintComponent.SetConstraintReferenceFrame` Constraint "Frame1" _returnvalue_2)
  (`PhysicsConstraintComponent.SetConstraintReferencePosition` Constraint "Frame1" _returnvalue_3)
  (bind _outactors (`KismetSystemLibrary.SphereOverlapActors` _returnvalue_3 (`self.Radius`) (`|MakeArray` "ObjectTypeQuery2" "ObjectTypeQuery4" "ObjectTypeQuery3" "ObjectTypeQuery5" "ObjectTypeQuery6" :!type "EObjectTypeQuery Enum") null (`|MakeArray` _returnvalue)))
  (`|ExecutionSequence`
    (:`then_0`
      (for _array_element _outactors
        (`PhysicsConstraintComponent.SetConstrainedComponents` Constraint (`Actor.GetComponentByClass` _returnvalue "/Script/Engine.MeshComponent") "None" (`Actor.GetComponentByClass` _array_element "/Script/Engine.MeshComponent") "None")))
    (:`then_1`
      (`self.HandleTackleStarted`))))